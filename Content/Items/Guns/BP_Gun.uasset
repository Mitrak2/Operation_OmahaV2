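; BP_Gun is an interactable gun item that the player can pick up, drop and fire.
; A Dropped/Equipped state, starting as Dropped, toggles mesh physics and the collision profiles of the sphere and mesh, resetting the mesh transform when equipped.
; Firing spawns a bullet and muzzle flash at the muzzle socket, aiming the bullet toward a far point along the camera's forward vector rather than using a trace.
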(event `self.ReceiveBeginPlay`
  (`self.SetGunState` "NewEnumerator0"))

(event `/Game/InteractionInterface/InteractionInterface.OnInteracted`
  (params (Player :type "/Game/AnimStarterPack/Ue4ASP_Character Object Reference"))
  (`/Game/AnimStarterPack/Ue4ASP_Character.Pick Up Gun` Player self)
  (`self.SetGunState` "NewEnumerator1"))

(fn `Drop`
  (`self.SetGunState` "NewEnumerator0"))

(fn `Fire`
  (params (PlayerCamera :type "CameraComponent Object Reference"))
  (bind _returnvalue (`SceneComponent.GetSocketLocation` (`self.SkeletalMesh`) "b_gun_muzzleflash"))
  (`|SpawnActorFromClass` "/Game/Items/Bullet/BP_Bullet.BP_Bullet_C" (`KismetMathLibrary.MakeTransform` _returnvalue) "Undefined" "OverrideRootScale" null (* (`KismetMathLibrary.Normal` (- (+ (`SceneComponent.K2_GetComponentLocation` PlayerCamera) (* (`SceneComponent.GetForwardVector` PlayerCamera) 10000.0)) _returnvalue)) 10000.0) null)
  (`|SpawnActorFromClass` "/Game/Items/Bullet/BP_MuzzleFlash.BP_MuzzleFlash_C" (`KismetMathLibrary.MakeTransform` _returnvalue) "Undefined" "OverrideRootScale" null null))

(fn `GetInteractionText`
  (returns (Text :type Text))
  (return "Pick Up"))

(fn `GetInteractionTextAttach`
  (returns (AttachComponent :type "SceneComponent Object Reference"))
  (return (`self.SkeletalMesh`)))

(fn `SetGunState`
  (params (NewGunState :type "/Game/Items/Guns/EGunState Enum" :default "NewEnumerator0"))
  (bind _skeletalmesh (`self.SkeletalMesh`))
  (bind _skeletalmesh_2 (`self.SkeletalMesh`))
  (bind _output_get (set `self.Gun State` NewGunState))
  (switch `/Game/Items/Guns/EGunState` _output_get
    (:`NewEnumerator0`
      (`PrimitiveComponent.SetCollisionProfileName` (`self.Sphere`) "OverlapAllDynamic" true)
      (`PrimitiveComponent.SetSimulatePhysics` _skeletalmesh_2 true)
      (`PrimitiveComponent.SetCollisionProfileName` _skeletalmesh_2 "DroppedGun" true))
    (:`NewEnumerator1`
      (`PrimitiveComponent.SetCollisionProfileName` (`self.Sphere`) "NoCollision" true)
      (`PrimitiveComponent.SetSimulatePhysics` _skeletalmesh false)
      (`PrimitiveComponent.SetCollisionProfileName` _skeletalmesh "NoCollision" true)
      (`SceneComponent.ResetRelativeTransform` (`self.SkeletalMesh`)))))

(fn `UserConstructionScript`
  (`parent.UserConstructionScript`))