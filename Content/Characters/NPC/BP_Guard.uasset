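; BP_Guard is an NPC guard character that owns a spawned weapon and ragdolls when killed.
; On BeginPlay it spawns the weapon at the world origin and stores it without attaching it.
; The health component's death event fires once to enable mesh physics and disable capsule collision, and IsDead forwards to that component.
; Damage and state-change events are empty, and GetTeamid returns a fixed value.
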(event `self.ReceiveBeginPlay`
  ;[1 0 0] Нужен BP WEAPON!!!!!!!!!!!!!!!!!!!!
  (bind _returnvalue (`|SpawnActorFromClass` (`GameplayStatics.GetObjectClass` (`self.WeaponClass`)) (`KismetMathLibrary.MakeTransform` (0.0 0.0 0.0)) "AlwaysSpawn" "OverrideRootScale" self null))
  (set `self.NewVar` _returnvalue))

(event `self.BPC_HealthComponent.OnDamageTaken`)

(event `self.BPC_HealthComponent.OnDeath`
  (`/Engine/EditorBlueprintResources/StandardMacros.DoOnce` false
    (:`Completed`
      (`PrimitiveComponent.SetCollisionProfileName` (`self.Mesh`) "Ragdoll" true)
      (`SkeletalMeshComponent.SetAllBodiesSimulatePhysics` (`self.Mesh`) true)
      (`PrimitiveComponent.SetCollisionEnabled` (`self.CapsuleComponent`) "NoCollision"))))

(event `/Game/Blueprints/Component/BPI_AIHelper.ChangeState`
  (params (NewState :type "/Game/AI/IE_NPCState Enum" :default "NewEnumerator0")))

(fn `GetTeamid`
  (returns (IsPlayer :type Boolean))
  (return false))

(fn `IsDead`
  (returns (Dead :type Boolean))
  (return (`/Game/Blueprints/Component/BPC_HealthComponent.IsDead` (`self.BPC_HealthComponent`))))

(fn `UserConstructionScript`)